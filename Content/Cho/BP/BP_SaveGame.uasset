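; BP_SaveGame holds the game's score ranking in ScoreArr, apparently as a save game object judging by its name.
; AddRanking appends a new score entry, then calls Sort.
; Sort orders the entries by TotalScore from highest to lowest, using a hand-written nested-loop exchange sort that swaps array elements in place.
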(event Custom|Add%20Ranking
  (params (Score :type BP%20Score%20Struct%20Structure))
  (Utilities|Array|Add (Variables|Default|GetScoreArr) Score)
  (CallFunction|Sort))

(event Custom|Sort
  (bind _scorearr (Variables|Default|GetScoreArr))
  (for (_array_element _array_index) _scorearr
    (for _index (range _array_index (- (Utilities|Array|Length _scorearr) 1))
      (if (> (.TotalScore (Utilities|Struct|BreakBP_ScoreStruct (Utilities|Array|Get(acopy) (Variables|Default|GetScoreArr) _index))) (.TotalScore (Utilities|Struct|BreakBP_ScoreStruct _array_element)))
        (Utilities|Array|Swap (Variables|Default|GetScoreArr) _index _array_index)))))