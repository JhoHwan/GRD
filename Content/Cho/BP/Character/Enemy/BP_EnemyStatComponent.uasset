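; BP_EnemyStatComponent holds an enemy's max HP, attack and current HP, and handles the damage it takes.
; SetStat copies max HP and attack from the passed-in data and fills HP to max.
; All HP changes route through SetHp, which clamps to the valid range and broadcasts OnHpChanged.
; ApplyDamage subtracts non-negative damage through SetHp and fires OnHpZero whenever HP is at zero afterward.
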(event Custom|Set%20Stat
  (params (InData :type BP%20Enemy%20Level%20Data%20Structure))
  (bind (_maxhp _attack) (Utilities|Struct|BreakBP_EnemyLevelData InData))
  (Variables|Default|SetMaxHp _maxhp)
  (Variables|Default|SetAttack _attack)
  (CallFunction|SetHp (Variables|Default|GetMaxHp)))

(event Custom|Apply%20Damage
  (params (InDamage :type Float%20%28double-precision%29))
  (CallFunction|SetHp (- (Variables|Default|GetCurrentHp) (Math|Float|Clamp(Float) InDamage 0.0 InDamage)))
  (if (<= (Variables|Default|GetCurrentHp) 0.0)
    (Default|CallOnHpZero)))

(event Custom|Set%20Hp
  (params (New%20Hp :type Float%20%28double-precision%29))
  (Variables|Default|SetCurrentHp (Math|Float|Clamp(Float) New%20Hp 0.0 (Variables|Default|GetMaxHp)))
  (Default|CallOnHpChanged (Variables|Default|GetCurrentHp)))