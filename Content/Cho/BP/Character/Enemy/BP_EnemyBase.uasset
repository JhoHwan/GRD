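; BP_EnemyBase is an enemy character base that handles damage, an HP bar widget and death.
; Incoming damage goes to its Stat component while HP remains, and SetWidget initializes the bar's maximum and binds Stat's HP-changed and HP-zero events.
; Dead stops the AIC_Base AI, plays the death montage and disables capsule collision.
; A montage notify freezes the pose, then the actor is destroyed after a short delay.
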(event Custom|Set%20Widget
  (bind _stat (Variables|Default|GetStat))
  (Default|SetMaxHp (Variables|Default|GetWB%20Enemy%20Hp%20Bar) (Variables|/Game/Cho/BP/Character/Enemy/BP_EnemyStatComponent.BP_EnemyStatComponent_C|GetMaxHp (Variables|Default|GetStat)))
  (EventDispatchers|BindEventtoOnHpChanged _stat (EventDispatchers|CreateEvent (Variables|Default|GetWB%20Enemy%20Hp%20Bar) :!event UpdateHp))
  (EventDispatchers|BindEventtoOnHpZero _stat (EventDispatchers|CreateEvent :!event Custom|Dead)))

(event Custom|Dead
  (bind _asaic_base (Utilities|Casting|CastToAIC_Base (AI|GetAIController self)))
  (Default|StopAi _asaic_base)
  (Animation|Montage|PlayMontage (Variables|Character|GetMesh) (Variables|Default|GetDeadMontage)
    (:then
      (Collision|SetCollisionEnabled (Variables|Default|GetCapsuleComponent) "NoCollision"))
    (:OnNotifyBegin
      (Class|AnimInstance|MontagePause (Components|SkeletalMesh|GetAnimInstance (Variables|Character|GetMesh)) (Variables|Default|GetDeadMontage))
      (Utilities|FlowControl|Delay 2.0)
      (Actor|DestroyActor))))

(event EventBeginPlay
  (bind _aswb_enemy_hp_bar (Utilities|Casting|CastToWB_EnemyHpBar (UserInterface|GetWidget (Variables|Default|GetWidget))))
  (Variables|Default|SetWB%20Enemy%20Hp%20Bar _aswb_enemy_hp_bar))

(event Game|Damage|EventAnyDamage
  (params (Damage :type Float%20%28single-precision%29) (DamageType :type Damage%20Type%20Object%20Reference) (InstigatedBy :type Controller%20Object%20Reference) (DamageCauser :type Actor%20Object%20Reference))
  (if (> (Variables|/Game/Cho/BP/Character/Enemy/BP_EnemyStatComponent.BP_EnemyStatComponent_C|GetCurrentHp (Variables|Default|GetStat)) 0.0)
    (Default|ApplyDamage (Variables|Default|GetStat) Damage)))

(fn ConstructionScript)