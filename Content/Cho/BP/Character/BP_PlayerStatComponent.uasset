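; Player stat component that tracks level, HP, XP, attack and health regeneration, loading per-level values from DT_PlayerLevelData.
; Setting a level refills HP and resets XP; filling the XP bar levels up, capped at level 10, with overflow XP discarded.
; HP and XP setters clamp their values and fire change dispatchers, alongside events for level changes and HP reaching zero.
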(event Custom|Set%20Level
  (params (New%20Level :type Integer))
  (Variables|Stat|SetLevel New%20Level)
  (bind _returnvalue (Utilities|GetDataTableRow "/Game/Cho/DataTable/Character/Player/Level/DT_PlayerLevelData.DT_PlayerLevelData" (Utilities|String|StringToName (Utilities|String|Append "Level" (Utilities|String|ToString(Integer) (Variables|Stat|GetLevel)))))
    (:then
      (Variables|Default|SetPlayerLevelData _returnvalue)
      (Utilities|FlowControl|Sequence
        (:then_0
          (Variables|Stat|SetMaxHp (.MaxHp (Utilities|Struct|BreakBP_PlayerLevelData (Variables|Default|GetPlayerLevelData))))
          (Variables|Stat|SetHealthRegeneration (.HealthRegeneration (Utilities|Struct|BreakBP_PlayerLevelData (Variables|Default|GetPlayerLevelData))))
          (Variables|Stat|SetAttack (.Attack (Utilities|Struct|BreakBP_PlayerLevelData (Variables|Default|GetPlayerLevelData))))
          (Variables|Stat|SetMaxXp (.MaxXp (Utilities|Struct|BreakBP_PlayerLevelData (Variables|Default|GetPlayerLevelData)))))
        (:then_1
          (Default|CallOnLevelChanged (Variables|Stat|GetMaxHp) (Variables|Stat|GetMaxXp))
          (CallFunction|SetHp (Variables|Stat|GetMaxHp))
          (CallFunction|SetXp))))))

(event Custom|Set%20Xp
  (params (NewXp :type Integer))
  (Variables|Stat|SetCurrentXp (Math|Integer|Clamp(Integer) NewXp 0 (Variables|Stat|GetMaxXp)))
  (Default|CallOnXpChanged (Variables|Stat|GetCurrentXp)))

(event Custom|Get%20Xp
  (params (InXp :type Integer))
  ;[1 1 1] Comment
  (if (< (Variables|Stat|GetLevel) 10)
    (CallFunction|SetXp (+ (Math|Integer|Clamp(Integer) InXp 0 InXp) (Variables|Stat|GetCurrentXp)))
    (if (== (Variables|Stat|GetCurrentXp) (Variables|Stat|GetMaxXp))
      (CallFunction|LevelUp))))

(event Custom|Apply%20Damage
  (params (InDamage :type Float%20%28double-precision%29))
  (CallFunction|SetHp (- (Variables|Stat|GetCurrentHp) (Math|Float|Clamp(Float) InDamage 0.0 InDamage)))
  (if (<= (Variables|Stat|GetCurrentHp) 0.0)
    (Default|CallOnHpZero)))

(event Custom|Level%20Up
  (if (< (Variables|Stat|GetLevel) 10)
    (bind _result (Math|Integer|IncrementInt (Variables|Stat|GetLevel))
      (:%20%20
        (CallFunction|SetLevel _result)))))

(event Custom|Set%20Hp
  (params (New%20Hp :type Float%20%28double-precision%29))
  (Variables|Stat|SetCurrentHp (Math|Float|Clamp(Float) New%20Hp 0.0 (Variables|Stat|GetMaxHp)))
  (Default|CallOnHpChanged (Variables|Stat|GetCurrentHp)))