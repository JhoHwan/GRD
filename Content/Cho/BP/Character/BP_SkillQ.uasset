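; BP_SkillQ is a short-lived damage actor for the player's Q skill.
; On BeginPlay it starts a self-destruct timer, then computes damage from the owning BP_Player's Attack stat and the Q skill data entry for the current Q level.
; Its Collision component applies that damage to any BP_EnemyBase that begins overlapping it.
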(event OnComponentBeginOverlap(Collision)
  (params (OverlappedComponent :type Primitive%20Component%20Object%20Reference) (OtherActor :type Actor%20Object%20Reference) (OtherComp :type Primitive%20Component%20Object%20Reference) (OtherBodyIndex :type Integer) (bFromSweep :type Boolean) (SweepResult :type Hit%20Result%20Structure%20%28by%20ref%29))
  (bind _asbp_enemy_base (Utilities|Casting|CastToBP_EnemyBase OtherActor))
  (Game|Damage|ApplyDamage _asbp_enemy_base (Variables|Default|GetDamage) 0 0 "/Script/Engine.DamageType"))

(event Custom|Destroy
  (Actor|DestroyActor))

(event EventBeginPlay
  (Utilities|Time|SetTimerbyEvent (delegate Custom|Destroy) 1.5)
  (bind _asbp_player (Utilities|Casting|CastToBP_Player (Components|GetOwner)))
  (Variables|Default|SetDamage (* (Variables|/Game/Cho/BP/Character/BP_PlayerStatComponent.BP_PlayerStatComponent_C|GetAttack (Variables|/Game/Cho/BP/Character/BP_Player.BP_Player_C|GetStat _asbp_player)) (.attack (Utilities|Array|Get(acopy) (.qskill (Variables|/Game/Cho/BP/Character/BP_PlayerStatComponent.BP_PlayerStatComponent_C|GetPlayerSkillData (Variables|/Game/Cho/BP/Character/BP_Player.BP_Player_C|GetStat _asbp_player))) (Variables|/Game/Cho/BP/Character/BP_PlayerStatComponent.BP_PlayerStatComponent_C|GetQ%20Level (Variables|/Game/Cho/BP/Character/BP_Player.BP_Player_C|GetStat _asbp_player)))))))

(fn ConstructionScript)