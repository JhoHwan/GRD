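; Blueprint function library of shared getters for the game's core references: game mode, player controller, player character and in-game HUD.
; The game mode getter casts the current game mode to BP_GameModeDefault.
; The controller getter returns that game mode's stored PlayerController if valid, otherwise casts player controller 0 to BP_CharacterController.
; The character and HUD getters read their references from that controller.
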(fn GetPlayerControllerRef
  (if (Utilities|IsValid (Variables|/Game/Cho/BP/BP_GameModeDefault.BP_GameModeDefault_C|GetPlayer%20Controller (CallFunction|GetGameModeRef)))
    (return (Variables|/Game/Cho/BP/BP_GameModeDefault.BP_GameModeDefault_C|GetPlayer%20Controller (CallFunction|GetGameModeRef)))
    (else
      (bind _asbp_character_controller (Utilities|Casting|CastToBP_CharacterController (Game|GetPlayerController 0)))
      (return _asbp_character_controller))))

(fn GetGameModeRef
  (bind _asbp_game_mode_default (Utilities|Casting|CastToBP_GameModeDefault (Game|GetGameMode))
    (:then
      _)
    (:CastFailed
      _))
  (return _asbp_game_mode_default))

(fn GetPlayerCharacterRef
  (return (Variables|/Game/Cho/BP/Character/BP_CharacterController.BP_CharacterController_C|GetPlayerCharacter (CallFunction|GetPlayerControllerRef))))

(fn GetinGameHUDRef
  (return (Variables|/Game/Cho/BP/Character/BP_CharacterController.BP_CharacterController_C|GetInGameHUD (CallFunction|GetPlayerControllerRef))))