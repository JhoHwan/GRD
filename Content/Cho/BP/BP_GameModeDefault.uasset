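; Default game mode that runs Story or Record play, chosen by the game instance's GameType, with enemy spawning and HUD updates.
; Story chains timed DataTable waves, spawning groups at random BP_Spawner points and showing a win screen once late-wave enemies are cleared.
; Record counts survival time into score, spawns enemies with a shrinking interval, has a boss spawn event, and saves rankings on game over.
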(event Custom|Update%20TImer
  (bind _time (Variables|Default|GetTime))
  ;[1 1 1] Game Timer
  (Math|Integer|DecrementInt (Variables|Default|GetTime)
    (:%20%20
      (Class|IHUD|UpdateTImer(Message) (Variables|Default|GetInGameHUD) _time)
      (if (<= _time 0)
        (Utilities|Time|PauseTimerbyHandle (stale Custom|Play%20Timer _returnvalue))))))

(event Custom|Play%20Timer
  (params (Time :type Integer))
  ;[1 1 1] Game Timer
  (bind _returnvalue (Utilities|Time|SetTimerbyEvent (delegate Custom|Update%20TImer) 1.0 true))
  (bind _output_get (Variables|Default|SetTime Time))
  (Class|IHUD|UpdateTImer(Message) (Variables|Default|GetInGameHUD) _output_get))

(event Custom|WinGame
  (bind _returnvalue (UserInterface|CreateWidget "/Game/Cho/BP/WidgetBP/HUD/WB_Result.WB_Result_C"))
  (Default|SetClear _returnvalue true)
  (UserInterface|Viewport|AddtoViewport _returnvalue 0))

(event Custom|Enemy%20Die
  (bind _result (Math|Integer|DecrementInt (Variables|Enemy|GetEnemyNum))
    (:%20%20
      (Class|IHUD|UpdateEnemyCount(Message) (Variables|Default|GetInGameHUD) _result)
      (if (and (>= (Variables|Default|GetCurrentWave) 5) (== (Variables|Enemy|GetEnemyNum) 0))
        (Utilities|FlowControl|Delay 3.0)
        (CallFunction|WinGame)))))

(event Custom|Create%20HUD
  (Variables|Default|GetInGameHUD
    (:then
      _)
    (:else
      (bind _returnvalue (UserInterface|CreateWidget "/Game/Cho/BP/WidgetBP/HUD/WB_HUD.WB_HUD_C"))
      (Variables|Default|SetInGameHUD _returnvalue)))
  (UserInterface|Viewport|AddtoViewport (Variables|Default|GetInGameHUD) 0))

(event Custom|Spawn%20Enemy
  (params (NewParam :type BP%20Enemy%20Base%20Class%20Reference))
  (bind _returnvalue (Game|SpawnActorfromClass NewParam (Transformation|GetActorTransform (.OutItem (Utilities|Array|Random (Variables|Enemy|GetSpawners)))) "AdjustIfPossibleButAlwaysSpawn" "MultiplyWithRoot" 0 0))
  (Pawn|SpawnDefaultController _returnvalue)
  (bind _result (Math|Integer|IncrementInt (Variables|Enemy|GetEnemyNum))
    (:%20%20
      (Class|IHUD|UpdateEnemyCount(Message) (Variables|Default|GetInGameHUD) _result)
      (EventDispatchers|BindEventtoOnHpZero (Variables|/Game/Cho/BP/Character/Enemy/BP_EnemyBase.BP_EnemyBase_C|GetStat _returnvalue) (delegate Custom|Enemy%20Die)))))

(event Custom|Start%20Story%20Mode
  (CallFunction|CreateHUD)
  (CallFunction|PlayTimer))

(event Custom|Create%20Tuto%20Widget
  (bind _returnvalue (UserInterface|CreateWidget "/Game/Cho/BP/WidgetBP/Tutorial/WBP_TutorialText.WBP_TutorialText_C"))
  (UserInterface|Viewport|AddtoViewport _returnvalue 0))

(event Custom|Start%20New%20Wave
  (bind _returnvalue (Utilities|GetDataTableRow "/Game/Cho/DataTable/Wave/DT_Wave.DT_Wave" (Utilities|String|StringToName (Utilities|String|Append "Wave" (Utilities|String|ToString(Integer) (Variables|Default|GetCurrentWave)))))
    (:then
      (Variables|Default|SetWave (.SpawnGroup (Utilities|Struct|BreakWavesStruct _returnvalue)))
      (bind _output_get (Variables|Default|SetWave%20Time (.WaveTime (Utilities|Struct|BreakWavesStruct _returnvalue))))
      (CallFunction|PlayTimer _output_get)
      (CallFunction|SpawnEnemyGroup)
      (Math|Integer|IncrementInt (Variables|Default|GetCurrentWave)
        (:%20%20
          (Utilities|Time|SetTimerbyEvent (EventDispatchers|CreateEvent :!event Custom|Start%20New%20Wave) (Math|Conversions|ToFloat(Integer) (Variables|Default|GetWave%20Time))))))
    (:RowNotFound
      (Variables|Default|SetWaveFinish true))))

(event Custom|SpawnEnemyGroup
  (bind _wave (Variables|Default|GetWave))
  (bind _output (Utilities|Array|Get(acopy) _wave))
  (bind _enemies (Utilities|Struct|BreakSpawnGroupStruct _output))
  (for _array_element _enemies
    (CallFunction|SpawnEnemy _array_element)
    (Utilities|Array|RemoveIndex _enemies))
  (Utilities|Array|RemoveIndex (Variables|Default|GetWave))
  (Utilities|Time|SetTimerbyEvent (delegate Custom|Spawn%20Next%20Enemy%20Group) 3.0))

(event Custom|Check%20Current%20Wave
  (if (Utilities|Array|IsValidIndex (Variables|Default|GetWave))
    (CallFunction|SpawnEnemyGroup)))

(event Custom|Spawn%20Next%20Enemy%20Group
  (CallFunction|CheckCurrentWave))

(event EventBeginPlay
  (Audio|SpawnSound2D "/Game/CY/sound/loop4.loop4" 1.0 1.0 0.0 0)
  (Variables|Player|SetPlayer%20Controller (CallFunction|GetPlayerControllerRef))
  (CallFunction|CreateHUD)
  (bind _outactors (Actor|GetAllActorsOfClass "/Game/Cho/BP/BP_Spawner.BP_Spawner_C"))
  (Variables|Enemy|SetSpawners _outactors)
  (switch Utilities|FlowControl|Switch|SwitchonEGameType (Variables|/Game/Cho/BP/BP_GameInstance.BP_GameInstance_C|GetGameType (CallFunction|GetMyGameInstance))
    (:NewEnumerator1
      (CallFunction|StartStoryMode)
      (CallFunction|StartNewWave))
    (:NewEnumerator2
      (CallFunction|StartRecordMode))))

(event Custom|Update%20Record%20Timer
  (Math|Integer|IncrementInt (Variables|Default|GetTime)
    (:%20%20
      (Class|IHUD|UpdateTImer(Message) (Variables|Default|GetInGameHUD) (Variables|Default|GetTime))
      (CallFunction|AddScore 7))))

(event Custom|Start%20Record%20Timer
  (Utilities|Time|SetTimerbyEvent (delegate Custom|Update%20Record%20Timer) 1.0 true)
  (bind _output_get (Variables|Default|SetTime 0))
  (Class|IHUD|UpdateTImer(Message) (Variables|Default|GetInGameHUD) _output_get))

(event Custom|Add%20Score
  (params (A :type Integer))
  (bind _output_get (Variables|Default|SetScore (+ A (Variables|Default|GetScore))))
  (Default|SetScore (Variables|Default|GetInGameHUD) _output_get))

(event Custom|Start%20Record%20Mode
  (bind _returnvalue (Utilities|GetDataTableRow "/Game/Cho/DataTable/Wave/DT_RecordStart.DT_RecordStart" "NewRow")
    (:then
      (Variables|Default|SetWave (.SpawnGroup (Utilities|Struct|BreakWavesStruct _returnvalue)))
      (bind _returnvalue_2 (Utilities|GetDataTableRow "/Game/Cho/DataTable/Wave/DT_RecordWave.DT_RecordWave" "NewRow")
        (:then
          (Variables|Record|SetRecord%20Wave (.SpawnGroup (Utilities|Struct|BreakWavesStruct _returnvalue_2)))
          (bind _output_get (Variables|Default|SetWave%20Time (.WaveTime (Utilities|Struct|BreakWavesStruct _returnvalue))))
          (CallFunction|PlayTimer _output_get)
          (CallFunction|RSpawnEnemyGroup)
          (CallFunction|StartRecordTimer)
          (Utilities|Time|SetTimerbyEvent (EventDispatchers|CreateEvent :!event Custom|Boss%20Timer) 3e+01 true))))))

(event Custom|Boss%20Timer
  (CallFunction|SpawnEnemy "/Game/Cho/BP/Character/Enemy/BP_Boss.BP_Boss_C"))

(event Custom|Game%20Over
  (bind _mygameinstance (CallFunction|GetMyGameInstance))
  (bind _score (Variables|Default|GetScore))
  (bind _time (Variables|Default|GetTime))
  (bind _returnvalue (* _time 7))
  (if (Utilities|Enum|Equal(Enum) (Variables|/Game/Cho/BP/BP_GameInstance.BP_GameInstance_C|GetGameType _mygameinstance) "NewEnumerator2")
    (Default|AddRanking (Variables|/Game/Cho/BP/BP_GameInstance.BP_GameInstance_C|GetSaveGameRef _mygameinstance) (Utilities|Struct|MakeBP_ScoreStruct "UNKOWN" _returnvalue (- _score _returnvalue) _score))
    (Default|SaveRank _mygameinstance)))

(event Custom|R%20Spawn%20enemy%20group
  (if (> (Variables|Default|GetRecordSpawnTime) 5.0)
    (Variables|Default|SetRecordSpawnTime (- (Variables|Default|GetRecordSpawnTime) 1.5)))
  (Utilities|Time|SetTimerbyEvent (EventDispatchers|CreateEvent :!event Custom|R%20Spawn%20enemy%20group) (Variables|Default|GetRecordSpawnTime))
  (for _array_element (Utilities|Struct|BreakSpawnGroupStruct (Utilities|Array|Get(acopy) (Variables|Record|GetRecord%20Wave)))
    (CallFunction|SpawnEnemy _array_element))
  (Utilities|Time|SetTimerbyEvent (delegate Custom|R%20Spawn%20next%20enemy%20group) 3.0)
  (for _array_element_2 (Utilities|Struct|BreakSpawnGroupStruct (Utilities|Array|Get(acopy) (Variables|Record|GetRecord%20Wave) 1))
    (CallFunction|SpawnEnemy _array_element_2)))

(event Custom|R%20Spawn%20next%20enemy%20group)

(fn ConstructionScript)