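; BP_Sword is a sword actor in the main character folder that bursts on impact, apparently part of a Q skill given its Niagara effect name.
; On BeginPlay it plays a 2D sound and spawns a scaled-up emitter at its own transform.
; When its box component hits something, it fires a radial force impulse, spawns the Niagara effect and a sound at the hit location, then destroys itself.
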(event OnComponentHit(Box)
  (params (HitComponent :type Primitive%20Component%20Object%20Reference) (OtherActor :type Actor%20Object%20Reference) (OtherComp :type Primitive%20Component%20Object%20Reference) (NormalImpulse :type Vector :default "0, 0, 0") (Hit :type Hit%20Result%20Structure%20%28by%20ref%29))
  (bind _location (Collision|BreakHitResult Hit))
  (Class|RadialForceComponent|FireImpulse (Variables|Default|GetRadialForce))
  (Niagara|SpawnSystematLocation "/Game/CY/VFX/NS_SkillQ/NS_SkillQ.NS_SkillQ" _location)
  (Audio|PlaySoundatLocation 0 _location "0, 0, 0" 1.0 1.0 0.0 0 0 0 0)
  (Actor|DestroyActor))

(event EventBeginPlay
  (Audio|PlaySound2D 0 1.0 1.0 0.0 0 0)
  (Effects|SpawnEmitteratLocation "/Game/esset/Action_FX/ParticleSystems/Magic_Bullet/Shoot.Shoot" (Transformation|GetActorLocation) (Transformation|GetActorRotation) "3.000000,3.000000,3.000000"))

(event Collision|EventActorBeginOverlap
  (params (OtherActor :type Actor%20Object%20Reference)))

(event EventTick
  (params (DeltaSeconds :type Float%20%28single-precision%29)))

(fn ConstructionScript)