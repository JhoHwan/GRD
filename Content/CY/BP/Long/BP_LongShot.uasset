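; BP_LongShot is the shot actor owned by BP_Long, apparently a ranged attacker, that damages the player on contact.
; On spawn it plays a sound, takes damage from the owner's Attack stat, flashes a brief muzzle emitter and self-destructs after a few seconds.
; Box overlap with BP_Player fires a radial impulse, spawns hit particles and sound, applies damage and destroys the shot.
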(event OnComponentBeginOverlap(Box)
  (params (OverlappedComponent :type Primitive%20Component%20Object%20Reference) (OtherActor :type Actor%20Object%20Reference) (OtherComp :type Primitive%20Component%20Object%20Reference) (OtherBodyIndex :type Integer) (bFromSweep :type Boolean) (SweepResult :type Hit%20Result%20Structure%20%28by%20ref%29))
  (bind _asbp_player (Utilities|Casting|CastToBP_Player OtherActor))
  (CallFunction|CreateEffect (+ (Transformation|GetActorLocation _asbp_player) "0.000000,0.000000,5.000000"))
  (Game|Damage|ApplyDamage _asbp_player (Variables|Default|GetDamage) 0 0)
  (Actor|DestroyActor))

(event EventBeginPlay
  (Audio|PlaySound2D 0 1.0 1.0 0.0 0 0)
  (bind _asbp_long (Utilities|Casting|CastToBP_Long (Components|GetOwner)))
  (Variables|Default|SetDamage (Variables|/Game/Cho/BP/Character/Enemy/BP_EnemyStatComponent.BP_EnemyStatComponent_C|GetAttack (Variables|/Game/Cho/BP/Character/Enemy/BP_EnemyBase.BP_EnemyBase_C|GetStat _asbp_long)))
  (bind _returnvalue (Effects|SpawnEmitteratLocation "/Game/esset/Action_FX/ParticleSystems/MuzzleFlash/P_MuzzleFlash.P_MuzzleFlash" (+ (Transformation|GetActorLocation) (* (Transformation|GetActorForwardVector) 4e+01)) (Transformation|GetActorRotation)))
  (Utilities|FlowControl|Delay 0.1)
  (Components|DestroyComponent _returnvalue)
  (Utilities|FlowControl|Delay 3.0)
  (Actor|DestroyActor))

(event Collision|EventActorBeginOverlap
  (params (OtherActor :type Actor%20Object%20Reference)))

(event EventTick
  (params (DeltaSeconds :type Float%20%28single-precision%29)))

(fn ConstructionScript)

(fn CreateEffect
  (params (Player%20Location :type Vector))
  (Class|RadialForceComponent|FireImpulse (Variables|Default|GetRadialForce))
  (Effects|SpawnEmitteratLocation "/Game/esset/Action_FX/ParticleSystems/MuzzleFlash/P_Hit2_1Spawn.P_Hit2_1Spawn" Player%20Location)
  (Audio|PlaySoundatLocation 0 Player%20Location "0, 0, 0" 1.0 1.0 0.0 0 0 0 0))

(fn SetDamage
  (params (Damage :type Float%20%28double-precision%29))
  (Variables|Default|SetDamage Damage))